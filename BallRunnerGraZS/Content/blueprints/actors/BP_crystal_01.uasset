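; BP_crystal_01 is a pickup crystal actor that flies to player 0's pawn, shrinks, dims its point light, then destroys itself.
; A sphere overlap plays a timeline whose three tracks drive location, scale and intensity lerps from current values each update.
; SetProperties caches starting values, but the lerps never read them.
; The IsPlayer check's comparison is unconnected, so any overlapping actor triggers it.
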(event `self.Sphere.OnComponentBeginOverlap`
  (params (OverlappedComponent :type "PrimitiveComponent Object Reference") (OtherActor :type "Actor Object Reference") (OtherComp :type "PrimitiveComponent Object Reference") (OtherBodyIndex :type Integer) (bFromSweep :type Boolean) (SweepResult :type "HitResult Structure (by ref)"))
  (`self.isPlayer` OtherActor)
  (`self.SetProperties`)
  (bind (_direction _lerpmovement _lerpscale _lerplight) (`Timeline|CrystalTimeMovement`) ; crystal_movement
    (:`Update`
      (`self.LerpLocation` _lerpmovement)
      (`self.LerpScale` _lerpscale)
      (`self.LerpLight` _lerplight))
    (:`Finished`
      (`self.K2_DestroyActor`))))

(fn `LerpLight`
  (params (Alpha :type "Float (double-precision)"))
  (bind _pointlight (`self.PointLight`))
  (`LightComponent.SetIntensity` _pointlight (`KismetMathLibrary.Lerp` (`LightComponentBase.Intensity` _pointlight) 0.0 Alpha)))

(fn `LerpLocation`
  (params (Alpha :type "Float (double-precision)"))
  (`self.K2_SetActorLocation` (`KismetMathLibrary.VLerp` (`self.K2_GetActorLocation`) (`self.K2_GetActorLocation` (`GameplayStatics.GetPlayerPawn` 0)) Alpha)))

(fn `LerpScale`
  (params (Alpha :type "Float (double-precision)"))
  (`self.SetActorScale3D` (`KismetMathLibrary.VLerp` (`self.GetActorScale3D`) (0.0 0.0 0.0) Alpha)))

(fn `SetProperties`
  (set `self.CrystalLocation` (`self.K2_GetActorLocation`))
  (set `self.CrystalScale` (`self.GetActorScale3D`))
  (set `self.CrystalIntensity` (`LightComponentBase.Intensity` (`self.PointLight`))))

(fn `UserConstructionScript`)